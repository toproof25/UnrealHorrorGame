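; Monster character Blueprint with PawnSensing, intended to turn toward noises and chase the player through AIMoveTo.
; Hearing stores the noise location for a smoothed turn, and a timed line-of-sight trace is meant to end the chase when blocked.
; Tick and OnSeePawn are empty, leaving the chase, trace and turn logic disconnected.
; Idle, walk and run events set MaxCustomMovementSpeed, and debug prints and boxes remain.
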(event `ForceIdle`
  (set `CharacterMovementComponent.MaxCustomMovementSpeed` 0.0 (`self.CharacterMovement`)))

(event `ForceWalk`
  (set `CharacterMovementComponent.MaxCustomMovementSpeed` 150.0 (`self.CharacterMovement`)))

(event `ForceRun`
  (set `CharacterMovementComponent.MaxCustomMovementSpeed` 400.0 (`self.CharacterMovement`)))

(event `FollowPlayer`
  ;[1 1 1] 폰 발견 시 추격하는 이벤트
  (if (`self.Is FollowPlayer`)
    (`|AIMoveTo` self (0.0 0.0 0.0) (`GameplayStatics.GetPlayerController` 0) 200.0
      (:`OnSuccess`
        (set `self.Is FollowPlayer` false)
        (`KismetSystemLibrary.Delay` 2.0)))))

(event `self.PawnSensing.OnSeePawn`
  (params (Pawn :type "Pawn Object Reference")))

(event `HearNoise`
  (bind _returnvalue (`SceneComponent.K2_GetComponentRotation` (`self.CapsuleComponent`)))
  (bind _returnvalue_2 (`SceneComponent.K2_GetComponentRotation` (`self.CapsuleComponent`)))
  (bind (_returnvalue_x _returnvalue_y) (`KismetMathLibrary.BreakVector` (`KismetMathLibrary.Vector_GetAbs` (- (`KismetMathLibrary.FindLookAtRotation` (`KismetMathLibrary.Conv_RotatorToVector` _returnvalue) (`self.HearLocation`)) _returnvalue))))
  ;[1 1 1] 소리나는 방향 바라보는 이벤트
  (`self.K2_SetActorRotation` (`KismetMathLibrary.RInterpTo` _returnvalue_2 (`KismetMathLibrary.FindLookAtRotation` (`KismetMathLibrary.Conv_RotatorToVector` _returnvalue_2) (`self.HearLocation`)) (`GameplayStatics.GetWorldDeltaSeconds`) 1.0))
  (`KismetSystemLibrary.PrintString` "노이즈 발생")
  (if (and (<= _returnvalue_x 0.3) (<= _returnvalue_y 0.3))
    (set `self.Is HearNoise` false)
    (`KismetSystemLibrary.PrintString` "회전 종료")))

(event `self.PawnSensing.OnHearNoise`
  (params (Instigator :type "Pawn Object Reference") (Location :type "Vector Structure (by ref)") (Volume :type "Float (single-precision)"))
  (set `self.HearLocation` Location)
  (if (not (`self.Is FollowPlayer`))
    (set `self.Is HearNoise` true)))

(event `self.ReceiveTick`
  (params (DeltaSeconds :type "Float (single-precision)")))

(fn `IsPlayerWall`
  (returns (Result :type Boolean))
  (bind _returnvalue (`SceneComponent.K2_GetComponentLocation` (`self.CapsuleComponent`)))
  ;[1 1 1] 몬스터에서 Pawn방향으로 Line 발사하고, Hit한 Actor 이름이 Pawn의 이름과 같다면 True, 아니라면 False를 반환
  (bind _outhit (`KismetSystemLibrary.LineTraceSingle` :`Start` _returnvalue :`End` (+ _returnvalue (* (`KismetMathLibrary.Normal` (- (`self.K2_GetActorLocation` (`GameplayStatics.GetPlayerPawn` 0)) (`self.K2_GetActorLocation`))) 7500.0)) :`TraceChannel` "TraceTypeQuery1" :`DrawDebugType` "ForOneFrame"))
  (bind (_bblockinghit _binitialoverlap _time _distance _location _impactpoint _normal _impactnormal _physmat _hitactor) (`GameplayStatics.BreakHitResult` _outhit))
  (`KismetSystemLibrary.DrawDebugBox` _location (10.0 10.0 10.0) (struct :`G` 1.0 :`B` 0.215291 :`A` 1.0) (struct) 10.0)
  (`KismetSystemLibrary.PrintString` (`KismetSystemLibrary.GetDisplayName` _hitactor))
  (return (== (`GameplayStatics.GetPlayerPawn` 0) _hitactor)))

(fn `PlayerOrWall`
  (params (B :type "Float (double-precision)"))
  ;[1 1 1] 폰을 발견 시 5초마다 Line발사하여 Pawn이면 계속 추격, Pawn이 아니면 이동을 멈춰서 추격을 종료
  (if (>= (`self.Timer`) 5.0)
    (set `self.Timer` 0.0)
    (bind _result (`self.IsPlayerWall`))
    (if (not _result)
      (set `self.Is FollowPlayer` false)
      (`NavMovementComponent.StopActiveMovement` (`self.CharacterMovement`)))
    (else
      (set `self.Timer` (+ (`self.Timer`) B)))))

(fn `UserConstructionScript`)