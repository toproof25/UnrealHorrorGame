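; BP_Item is a collectible item actor whose static mesh can be highlighted with an outline.
; ApplyOverlay sets an outliner overlay material on the mesh, and RemoveOverlay clears it by restoring an empty original material.
; When destroyed, it calls GetItem on BP_GameModeBase to register the pickup and prints a debug message.
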(event `self.ReceiveBeginPlay`
  (set `self.OriginalMaterial ` null)
  (set `self.OverlayMaterial` "/Game/Materials/Mat_Outliner.Mat_Outliner"))

(event `self.ReceiveDestroyed`
  (bind _asbp_game_mode_base (cast `/Game/Blueprints/GameModeBase/BP_GameModeBase` (`GameplayStatics.GetGameMode`)))
  (`/Game/Blueprints/GameModeBase/BP_GameModeBase.Get Item` _asbp_game_mode_base)
  (`KismetSystemLibrary.PrintString` "아이템 함수 실행하고 나는 사라진당"))

(fn `ApplyOverlay`
  (`MeshComponent.SetOverlayMaterial` (`self.StaticMesh`) (`self.OverlayMaterial`)))

(fn `RemoveOverlay`
  (`MeshComponent.SetOverlayMaterial` (`self.StaticMesh`) (`self.OriginalMaterial `)))

(fn `UserConstructionScript`)