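; Player pawn with camera-relative movement and look via Enhanced Input, a toggleable flashlight, and a test input that emits noise through PawnNoiseEmitter.
; Tick line-traces from the camera to apply or remove an overlay on the targeted BP_Item, initially seeded by GetActorOfClass.
; Mouse click runs a longer trace with a debug box, destroying nearby actors tagged "item" and setting the Item flag on BP_GameModeBase.
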(event `self.ReceiveBeginPlay`
  (`EnhancedInputSubsystemInterface.AddMappingContext` (pcsubsystem `EnhancedInputLocalPlayerSubsystem` (`GameplayStatics.GetPlayerController` 0)) "/Game/Blueprints/InputMappingContext/IMC_InputMappingContext.IMC_InputMappingContext" 0 (struct))
  (bind _returnvalue (`GameplayStatics.GetActorOfClass` "/Game/Blueprints/BP_Item.BP_Item_C"))
  (bind _output_get (set `self.CurrentlyTargetedItem` _returnvalue))
  (`KismetSystemLibrary.PrintString` (`KismetSystemLibrary.GetDisplayName` _output_get)))

(event `EnhancedInput|/Game/Blueprints/InputActions/IA_TestNoice`
  (params (ActionValue :type Boolean) (ElapsedSeconds :type "Float (double-precision)") (TriggeredSeconds :type "Float (double-precision)") (InputAction :type "InputAction Object Reference" :default "/Game/Blueprints/InputActions/IA_TestNoice.IA_TestNoice"))
  ;[1 1 1] Test Noise Event
  (:`Started`
    (`PawnNoiseEmitterComponent.MakeNoise` (`self.PawnNoiseEmitter`) self 1.0 (`self.K2_GetActorLocation`))))

(event `EnhancedInput|/Game/Blueprints/InputActions/IA_InputActionForward`
  (params (ActionValue :type "Float (double-precision)") (ElapsedSeconds :type "Float (double-precision)") (TriggeredSeconds :type "Float (double-precision)") (InputAction :type "InputAction Object Reference" :default "/Game/Blueprints/InputActions/IA_InputActionForward.IA_InputActionForward"))
  ;[1 1 1] Move Forward or Backward & Right or Left
  (:`Triggered`
    (`self.AddMovementInput` (`KismetMathLibrary.GetForwardVector` (`KismetMathLibrary.MakeRotator` 0.0 0.0 (.yaw (`self.GetControlRotation`)))) ActionValue)))

(event `EnhancedInput|/Game/Blueprints/InputActions/IA_InputActionRight`
  (params (ActionValue :type "Float (double-precision)") (ElapsedSeconds :type "Float (double-precision)") (TriggeredSeconds :type "Float (double-precision)") (InputAction :type "InputAction Object Reference" :default "/Game/Blueprints/InputActions/IA_InputActionRight.IA_InputActionRight"))
  ;[1 1 1] Move Forward or Backward & Right or Left
  (:`Triggered`
    (`self.AddMovementInput` (`KismetMathLibrary.GetRightVector` (`KismetMathLibrary.MakeRotator` 0.0 0.0 (.yaw (`self.GetControlRotation`)))) ActionValue)))

(event `EnhancedInput|/Game/Blueprints/InputActions/IA_Look`
  (params (ActionValue :type "Float (double-precision)") (ElapsedSeconds :type "Float (double-precision)") (TriggeredSeconds :type "Float (double-precision)") (InputAction :type "InputAction Object Reference" :default "/Game/Blueprints/InputActions/IA_Look.IA_Look"))
  ;[1 1 1] Turn or Look
  (:`Triggered`
    (`self.AddControllerPitchInput` ActionValue)))

(event `EnhancedInput|/Game/Blueprints/InputActions/IA_Turn`
  (params (ActionValue :type "Float (double-precision)") (ElapsedSeconds :type "Float (double-precision)") (TriggeredSeconds :type "Float (double-precision)") (InputAction :type "InputAction Object Reference" :default "/Game/Blueprints/InputActions/IA_Turn.IA_Turn"))
  ;[1 1 1] Turn or Look
  (:`Triggered`
    (`self.AddControllerYawInput` ActionValue)))

(event `EnhancedInput|/Game/Blueprints/InputActions/IA_Light`
  (params (ActionValue :type Boolean) (ElapsedSeconds :type "Float (double-precision)") (TriggeredSeconds :type "Float (double-precision)") (InputAction :type "InputAction Object Reference" :default "/Game/Blueprints/InputActions/IA_Light.IA_Light"))
  ;[1 1 1] Light on/off
  (:`Started`
    (`SceneComponent.ToggleVisibility` (`self.flash`) ActionValue)))

(event `EnhancedInput|/Game/Blueprints/InputActions/IA_MouseClick`
  (params (ActionValue :type Boolean) (ElapsedSeconds :type "Float (double-precision)") (TriggeredSeconds :type "Float (double-precision)") (InputAction :type "InputAction Object Reference" :default "/Game/Blueprints/InputActions/IA_MouseClick.IA_MouseClick"))
  (bind _returnvalue (`GameplayStatics.GetPlayerCameraManager` 0))
  (bind _returnvalue_2 (`PlayerCameraManager.GetCameraLocation` _returnvalue))
  ;[1 1 1] Mouse Click Draw Debug Box
  (:`Started`
    (`KismetSystemLibrary.PrintString` "Pawn 마우스 이벤트")
    (bind (_outhit _returnvalue_3) (`KismetSystemLibrary.LineTraceSingle` _returnvalue_2 (+ _returnvalue_2 (* (`KismetMathLibrary.GetForwardVector` (`PlayerCameraManager.GetCameraRotation` _returnvalue)) 1500.0)) "TraceTypeQuery1"))
    (if _returnvalue_3
      (bind (_bblockinghit _binitialoverlap _time _distance _location _impactpoint _normal _impactnormal _physmat _hitactor) (`GameplayStatics.BreakHitResult` _outhit))
      (`KismetSystemLibrary.DrawDebugBox` _location (10.0 10.0 10.0) (struct :`R` 1.0 :`B` 0.646856 :`A` 1.0) (struct) 2.0)
      (if (`self.ActorHasTag` _hitactor "item")
        (if (<= _distance 150.0)
          (`self.K2_DestroyActor` _hitactor)
          (bind _asbp_game_mode_base (cast `/Game/Blueprints/GameModeBase/BP_GameModeBase` (`GameplayStatics.GetGameMode`)))
          (set `/Game/Blueprints/GameModeBase/BP_GameModeBase.item` true _asbp_game_mode_base))))))

(event `self.ReceiveTick`
  (params (DeltaSeconds :type "Float (single-precision)"))
  (bind _returnvalue (`GameplayStatics.GetPlayerCameraManager` 0))
  (bind _returnvalue_2 (`PlayerCameraManager.GetCameraLocation` _returnvalue))
  ;[1 1 1] 라인 발사
  (bind (_outhit _returnvalue_3) (`KismetSystemLibrary.LineTraceSingle` _returnvalue_2 (+ _returnvalue_2 (* (`KismetMathLibrary.GetForwardVector` (`PlayerCameraManager.GetCameraRotation` _returnvalue)) 500.0)) "TraceTypeQuery1"))
  ;[1 1 1] 발사된 라인에 닿은 액터가 아이템이면 아이템의 외각을 빛나게 설정, 아니면 복구
  (if _returnvalue_3
    (bind (_bblockinghit _binitialoverlap _time _distance _location _impactpoint _normal _impactnormal _physmat _hitactor) (`GameplayStatics.BreakHitResult` _outhit))
    (bind _asbp_item (cast `/Game/Blueprints/BP_Item` _hitactor)
      (:`then`
        (bind _output_get (set `self.CurrentlyTargetedItem` _asbp_item))
        (`/Game/Blueprints/BP_Item.ApplyOverlay` _output_get))
      (:`CastFailed`
        (if (not (== _hitactor (`self.CurrentlyTargetedItem`))) :!label _label
          (`/Game/Blueprints/BP_Item.RemoveOverlay` (`self.CurrentlyTargetedItem`)))))
    (else
      (goto _label))))

(fn `UserConstructionScript`)