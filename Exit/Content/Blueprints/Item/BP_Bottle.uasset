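; BP_Bottle is a throwable bottle item that shatters on impact and creates noise through the player.
; Fire launches the static mesh with a velocity-change impulse along the given forward vector and arms a thrown flag.
; The first Hit while armed clears the flag, passes the hit location to BP_Player's Noise, and spawns a ceramic destruction effect.
; It then hides the actor, plays a breaking sound, and destroys itself after a short delay.
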(event `self.ReceiveTick`
  (params (DeltaSeconds :type "Float (single-precision)")))

(event `self.ReceiveHit`
  (params (MyComp :type "PrimitiveComponent Object Reference") (Other :type "Actor Object Reference") (OtherComp :type "PrimitiveComponent Object Reference") (bSelfMoved :type Boolean) (HitLocation :type "Vector Structure") (HitNormal :type "Vector Structure") (NormalImpulse :type "Vector Structure") (Hit :type "HitResult Structure (by ref)"))
  (bind _audio (`self.Audio`))
  (if (`self.Is thrrow`)
    (set `self.Is thrrow` false)
    (bind _asbp_player (cast `/Game/Blueprints/BP_Player` (`GameplayStatics.GetPlayerPawn` 0)))
    (`/Game/Blueprints/BP_Player.Noise` _asbp_player HitLocation)
    (`GameplayStatics.SpawnEmitterAtLocation` "/Game/VFX/Realistic_Starter_VFX_Pack_Vol2/Particles/Destruction/P_Destruction_Ceramic.P_Destruction_Ceramic" HitLocation)
    (`self.SetActorHiddenInGame` true)
    (`AudioComponent.SetSound` _audio "/Game/Sounds/MSS_BottleBroken.MSS_BottleBroken")
    (`AudioComponent.Play` _audio 0.0)
    (`KismetSystemLibrary.Delay` 1.33)
    (`self.K2_DestroyActor`)))

(event `Fire`
  (params (ForwardVector :type "Vector Structure"))
  (`PrimitiveComponent.AddImpulse` (`self.StaticMesh`) (* ForwardVector 1500.0) "None" true)
  (set `self.Is thrrow` true))

(fn `UserConstructionScript`)