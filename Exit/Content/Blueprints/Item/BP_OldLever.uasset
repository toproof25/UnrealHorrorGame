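; BP_OldLever is an old lever item actor that can show or hide an outline highlight on its static mesh.
; BeginPlay caches Mat_Outliner as the overlay material and leaves the original empty, so ApplyOverlay sets the outline and RemoveOverlay clears it.
; The Destroyed event casts the game mode to BP_GameModeBase but takes no further action.
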(event `self.ReceiveBeginPlay`
  (set `self.OriginalMaterial ` null)
  (set `self.OverlayMaterial` "/Game/Materials/Mat_Outliner.Mat_Outliner"))

(event `self.ReceiveDestroyed`
  (cast `/Game/Blueprints/GameModeBase/BP_GameModeBase` (`GameplayStatics.GetGameMode`)))

(fn `ApplyOverlay`
  (`MeshComponent.SetOverlayMaterial` (`self.StaticMesh`) (`self.OverlayMaterial`)))

(fn `RemoveOverlay`
  (`MeshComponent.SetOverlayMaterial` (`self.StaticMesh`) (`self.OriginalMaterial `)))

(fn `UserConstructionScript`)