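; BP_Chain is a breakable chain actor that can be highlighted with an outline and broken.
; BeginPlay gathers ten chain components into an array, which ApplyOverlay and RemoveOverlay loop over to set or clear the Mat_Outliner overlay material.
; RemoveChain clears the outline, destroys Chain7 and the Box component, and plays a break sound and wood-destruction particles.
; An IsRemove flag then blocks further highlighting.
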(event `self.ReceiveBeginPlay`
  (set `self.Chains` (`|MakeArray` (`self.chain2`) (`self.chain9`) (`self.chain10`) (`self.chain8`) (`self.chain7`) (`self.chain6`) (`self.chain11`) (`self.chain4`) (`self.chain5`) (`self.chain3`)))
  (set `self.Original Matertial` null)
  (set `self.Overlay Matertial` "/Game/Materials/Mat_Outliner.Mat_Outliner"))

(event `RemoveChain`
  (bind _returnvalue (`self.K2_GetActorLocation`))
  (`self.RemoveOverlay`)
  (`ActorComponent.K2_DestroyComponent` (`self.chain7`))
  (`ActorComponent.K2_DestroyComponent` (`self.Box`))
  (set `self.is remove?` true)
  (`GameplayStatics.PlaySoundAtLocation` "/Game/Sounds/SOUND_ChainBroken.SOUND_ChainBroken" _returnvalue (struct) 1.0 1.0 0.0 "/Game/Sounds/SA_ZombieSound.SA_ZombieSound" null null null)
  (`GameplayStatics.SpawnEmitterAtLocation` "/Game/VFX/Realistic_Starter_VFX_Pack_Vol2/Particles/Destruction/P_Destruction_Wood.P_Destruction_Wood" (+ _returnvalue (100.0 0.0 0.0))))

(event `RemoveOverlay`
  (for _array_element (`self.Chains`)
    (`MeshComponent.SetOverlayMaterial` _array_element (`self.Original Matertial`))))

(event `ApplyOverlay`
  (if (not (`self.is remove?`))
    (for _array_element (`self.Chains`)
      (`MeshComponent.SetOverlayMaterial` _array_element (`self.Overlay Matertial`)))))

(fn `UserConstructionScript`)