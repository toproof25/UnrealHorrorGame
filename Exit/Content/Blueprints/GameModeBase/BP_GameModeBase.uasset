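; Game mode for a labyrinth game with a pursuing enemy, holding the main HUD, player lives and progress flags.
; Nearby enemy hits trigger blood and camera shake and decrement LifeCount; at zero a death sequence plays, then the game pauses until RestartEvent reloads the level.
; ActivateLever plays a lever sequence, and Last speeds up the cached enemy.
; Ending only clears the Item flag; its sequence-and-quit chain is disconnected.
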(event `Restart Event`
  ;[1 1 1] 게임 재시작
  (`GameplayStatics.OpenLevelBySoftObjectPtr` "/Game/Levels/LV_Labyrinth.LV_Labyrinth"))

(event `self.ReceiveBeginPlay`
  ;[1 1 1] UI
  (bind _returnvalue (`|CreateWidget` "/Game/Blueprints/Widget/WBP_MainWidget.WBP_MainWidget_C"))
  (`UserWidget.AddToViewport` _returnvalue 0)
  (`KismetSystemLibrary.Delay` 1.0)
  (bind _returnvalue_2 (`GameplayStatics.GetActorOfClass` "/Game/Blueprints/Enemy/BP_Enemy.BP_Enemy_C"))
  (bind _output_get (set `self.Enemy` _returnvalue_2))
  (`KismetSystemLibrary.PrintString` (`KismetSystemLibrary.GetDisplayName` _output_get) false))

(event `DeadEvent`
  ;[1 1 1] Dead시 시퀀스 실행 후 재시작
  (bind (_outactor _returnvalue) (`LevelSequencePlayer.CreateLevelSequencePlayer` "/Game/LevelSequence/DeadSequence.DeadSequence"))
  (`MovieSceneSequencePlayer.Play` _returnvalue)
  (`KismetSystemLibrary.Delay` (`TimeManagementBlueprintLibrary.Conv_QualifiedFrameTimeToSeconds` (`MovieSceneSequencePlayer.GetDuration` _returnvalue)))
  (bind _returnvalue_2 (`GameplayStatics.SetGamePaused` true))
  (set `PlayerController.bShowMouseCursor` _returnvalue_2 (`GameplayStatics.GetPlayerController` 0))
  (set `self.Restart` true))

(event `Ending`
  ;[1 1 1] 엔딩 시퀀스 실행 후 게임 종료
  (if (`self.item`)
    (set `self.item` false)))

(event `Activate Lever`
  ;[1 1 1] 레버 사용 시 문열리는 시퀀스 실행
  (set `self.lever` true)
  (`KismetSystemLibrary.PrintString` "Hello" false)
  (bind (_outactor _returnvalue) (`LevelSequencePlayer.CreateLevelSequencePlayer` "/Game/LevelSequence/LeverSequence.LeverSequence"))
  (`MovieSceneSequencePlayer.Play` _returnvalue))

(event `Hit Event`
  (params (Enemy :type "/Game/Blueprints/Enemy/BP_Enemy Object Reference"))
  (bind _returnvalue (`GameplayStatics.GetPlayerPawn` 0))
  ;[1 1 1] LifeCount만큼 맞으면 사망
  (if (<= (`self.GetDistanceTo` Enemy _returnvalue) 800.0)
    (`GameplayStatics.SpawnEmitterAtLocation` "/Game/VFX/Realistic_Starter_VFX_Pack_Vol2/Particles/Blood/P_Blood_Splat_Cone.P_Blood_Splat_Cone" (`self.K2_GetActorLocation` _returnvalue))
    (`GameplayStatics.PlayWorldCameraShake` "/Game/Blueprints/BP_CameraShake.BP_CameraShake_C" (`self.K2_GetActorLocation` (`GameplayStatics.GetPlayerCameraManager` 0)) 0.0 1000.0 3.0)
    (`KismetSystemLibrary.PrintString` "아야!" false)
    (set `self.LifeCount` (- (`self.LifeCount`) 1))
    (if (<= (`self.LifeCount`) 0)
      (`self.DeadEvent`))))

(event `Last`
  (set `self.lastEvent` true)
  (`/Game/Blueprints/Enemy/BP_Enemy.MaxSpeed` (`self.Enemy`)))

(fn `UserConstructionScript`)