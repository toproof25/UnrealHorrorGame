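; First-person player pawn for movement, flashlight and interaction with a key item, lever, bolt cutter, chain and throwable bottle.
; Tick line-traces from the camera to highlight interactables cached at BeginPlay with overlays.
; Clicking traces again to collect or activate them, updating BP_GameModeBase and emitting pawn noise for most actions.
; Bottles are grabbed with a PhysicsHandle, moved by a looping timer and fired along the camera direction on release.
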(event `self.ReceiveBeginPlay`
  ;[1 1 1] Input Mapping
  (`EnhancedInputSubsystemInterface.AddMappingContext` (pcsubsystem `EnhancedInputLocalPlayerSubsystem` (`GameplayStatics.GetPlayerController` 0)) "/Game/Blueprints/InputMappingContext/IMC_InputMappingContext.IMC_InputMappingContext" 0 (struct))
  ;[1 1 1] 레벨에 배치된 item, lever 액터를 미리 변수에 저장
  (bind _returnvalue (`GameplayStatics.GetActorOfClass` "/Game/Blueprints/Item/BP_Item.BP_Item_C"))
  (set `self.Item` _returnvalue)
  (bind _returnvalue_2 (`GameplayStatics.GetActorOfClass` "/Game/Blueprints/Item/BP_OldLever.BP_OldLever_C"))
  (set `self.Lever` _returnvalue_2)
  (bind _returnvalue_3 (`GameplayStatics.GetActorOfClass` "/Game/Blueprints/Item/BP_Chain.BP_Chain_C"))
  (set `self.chain` _returnvalue_3)
  (bind _returnvalue_4 (`GameplayStatics.GetActorOfClass` "/Game/Blueprints/Item/BP_BoltCutter.BP_BoltCutter_C"))
  (set `self.bolt cutter` _returnvalue_4))

(event `EnhancedInput|/Game/Blueprints/InputActions/IA_InputActionForward`
  (params (ActionValue :type "Float (double-precision)") (ElapsedSeconds :type "Float (double-precision)") (TriggeredSeconds :type "Float (double-precision)") (InputAction :type "InputAction Object Reference" :default "/Game/Blueprints/InputActions/IA_InputActionForward.IA_InputActionForward"))
  ;[1 1 1] Move Forward or Backward & Right or Left
  (:`Triggered`
    (`self.AddMovementInput` (`KismetMathLibrary.GetForwardVector` (`KismetMathLibrary.MakeRotator` 0.0 0.0 (.yaw (`self.GetControlRotation`)))) ActionValue)))

(event `EnhancedInput|/Game/Blueprints/InputActions/IA_InputActionRight`
  (params (ActionValue :type "Float (double-precision)") (ElapsedSeconds :type "Float (double-precision)") (TriggeredSeconds :type "Float (double-precision)") (InputAction :type "InputAction Object Reference" :default "/Game/Blueprints/InputActions/IA_InputActionRight.IA_InputActionRight"))
  ;[1 1 1] Move Forward or Backward & Right or Left
  (:`Triggered`
    (`self.AddMovementInput` (`KismetMathLibrary.GetRightVector` (`KismetMathLibrary.MakeRotator` 0.0 0.0 (.yaw (`self.GetControlRotation`)))) ActionValue)))

(event `EnhancedInput|/Game/Blueprints/InputActions/IA_Look`
  (params (ActionValue :type "Float (double-precision)") (ElapsedSeconds :type "Float (double-precision)") (TriggeredSeconds :type "Float (double-precision)") (InputAction :type "InputAction Object Reference" :default "/Game/Blueprints/InputActions/IA_Look.IA_Look"))
  ;[1 1 1] Turn or Look
  (:`Triggered`
    (`self.AddControllerPitchInput` ActionValue)))

(event `EnhancedInput|/Game/Blueprints/InputActions/IA_TestNoice`
  (params (ActionValue :type Boolean) (ElapsedSeconds :type "Float (double-precision)") (TriggeredSeconds :type "Float (double-precision)") (InputAction :type "InputAction Object Reference" :default "/Game/Blueprints/InputActions/IA_TestNoice.IA_TestNoice"))
  ;[1 1 1] Test Noise Event
)

(event `EnhancedInput|/Game/Blueprints/InputActions/IA_Turn`
  (params (ActionValue :type "Float (double-precision)") (ElapsedSeconds :type "Float (double-precision)") (TriggeredSeconds :type "Float (double-precision)") (InputAction :type "InputAction Object Reference" :default "/Game/Blueprints/InputActions/IA_Turn.IA_Turn"))
  ;[1 1 1] Turn or Look
  (:`Triggered`
    (`self.AddControllerYawInput` ActionValue)))

(event `PickedUp`
  (bind (_returnvalue_location _returnvalue_rotation) (`KismetMathLibrary.BreakTransform` (`SceneComponent.K2_GetComponentToWorld` (`self.Camera`))))
  (`KismetSystemLibrary.K2_SetTimerDelegate` (delegate `PickedUp`) 0.02 true true)
  (`PhysicsHandleComponent.SetTargetLocation` (`self.PhysicsHandle`) (+ _returnvalue_location (* (`KismetMathLibrary.GetForwardVector` _returnvalue_rotation) 200.0))))

(event `Noise`
  (params (Location :type "Vector Structure"))
  (`PawnNoiseEmitterComponent.MakeNoise` (`self.PawnNoiseEmitter`) self 1.0 Location))

(event `EnhancedInput|/Game/Blueprints/InputActions/IA_Light`
  (params (ActionValue :type Boolean) (ElapsedSeconds :type "Float (double-precision)") (TriggeredSeconds :type "Float (double-precision)") (InputAction :type "InputAction Object Reference" :default "/Game/Blueprints/InputActions/IA_Light.IA_Light"))
  ;[1 1 1] Light on/off
  (:`Started`
    (`SceneComponent.ToggleVisibility` (`self.flash`) ActionValue)))

(event `EnhancedInput|/Game/Blueprints/InputActions/IA_MouseClick`
  (params (ActionValue :type Boolean) (ElapsedSeconds :type "Float (double-precision)") (TriggeredSeconds :type "Float (double-precision)") (InputAction :type "InputAction Object Reference" :default "/Game/Blueprints/InputActions/IA_MouseClick.IA_MouseClick"))
  (bind _returnvalue (`GameplayStatics.GetPlayerCameraManager` 0))
  (bind _returnvalue_2 (`PlayerCameraManager.GetCameraLocation` _returnvalue))
  (:`Started`
    ;[1 1 1] Mouse Click Draw Debug Box
    (`KismetSystemLibrary.PrintString` "Pawn 마우스 이벤트" false)
    (bind (_outhit _returnvalue_3) (`KismetSystemLibrary.LineTraceSingle` :`Start` _returnvalue_2 :`End` (+ _returnvalue_2 (* (`KismetMathLibrary.GetForwardVector` (`PlayerCameraManager.GetCameraRotation` _returnvalue)) 200.0)) :`TraceChannel` "TraceTypeQuery1" :`DrawDebugType` "ForOneFrame"))
    ;[1 1 1] 마우스 클릭 시 액터가 Item or Lever이라면
    (if _returnvalue_3
      (bind (_bblockinghit _binitialoverlap _time _distance _location _impactpoint _normal _impactnormal _physmat _hitactor _hitcomponent) (`GameplayStatics.BreakHitResult` _outhit))
      (if (<= _distance 150.0)
        (`self.Get Item` _hitactor)
        (`self.Activate Lever` _hitactor)
        (`self.Activate Chain` _hitactor))
      ;[1 1 1] Grab and thrrow
      (bind _asbp_bottle (cast `/Game/Blueprints/Item/BP_Bottle` _hitactor))
      (set `self.bottle` _asbp_bottle)
      (`PhysicsHandleComponent.GrabComponentAtLocationWithRotation` (`self.PhysicsHandle`) _hitcomponent "None" (`SceneComponent.K2_GetComponentLocation` _hitcomponent) (`SceneComponent.K2_GetComponentRotation` _hitcomponent))
      (set `self.ObjectGrab` true)
      (`self.PickedUp`)))
  (:`Completed`
    ;[1 1 1] 소리 아이템을 들고 있으면 던지기
    (`KismetSystemLibrary.PrintString` "조룔죠룢" false)
    (if (`self.ObjectGrab`)
      (set `self.ObjectGrab` false)
      (`PhysicsHandleComponent.ReleaseComponent` (`self.PhysicsHandle`))
      (`/Game/Blueprints/Item/BP_Bottle.Fire` (`self.bottle`) (`KismetMathLibrary.GetForwardVector` (`PlayerCameraManager.GetCameraRotation` (`GameplayStatics.GetPlayerCameraManager` 0)))))))

(event `self.ReceiveTick`
  (params (DeltaSeconds :type "Float (single-precision)"))
  (bind _returnvalue (`GameplayStatics.GetPlayerCameraManager` 0))
  (bind _returnvalue_2 (`PlayerCameraManager.GetCameraLocation` _returnvalue))
  ;[1 1 1] 라인 발사
  (bind (_outhit _returnvalue_3) (`KismetSystemLibrary.LineTraceSingle` _returnvalue_2 (+ _returnvalue_2 (* (`KismetMathLibrary.GetForwardVector` (`PlayerCameraManager.GetCameraRotation` _returnvalue)) 500.0)) "TraceTypeQuery1"))
  ;[1 1 1] 발사된 라인에 닿은 액터가 아이템 or 레버면 외각을 빛나게 설정, 아니면 복구
  (if _returnvalue_3
    (bind (_bblockinghit _binitialoverlap _time _distance _location _impactpoint _normal _impactnormal _physmat _hitactor) (`GameplayStatics.BreakHitResult` _outhit))
    (`self.Is Item` _hitactor)
    (`self.Is Lever` _hitactor)
    (`self.Is Chain` _hitactor)
    (`self.Is BoltCutter` _hitactor)))

(fn `Activate Chain`
  (params (`Hit Actor` :type "Actor Object Reference"))
  (if (`self.Get Bolt Cutter`)
    (if (== `Hit Actor` (`self.chain`))
      (`/Game/Blueprints/Item/BP_Chain.RemoveChain` (`self.chain`))
      (bind _asbp_game_mode_base (cast `/Game/Blueprints/GameModeBase/BP_GameModeBase` (`GameplayStatics.GetGameMode`)))
      (set `/Game/Blueprints/GameModeBase/BP_GameModeBase.boltCutter` false _asbp_game_mode_base)
      (`self.Noise` (`self.K2_GetActorLocation`))
      (`/Game/Blueprints/GameModeBase/BP_GameModeBase.Last` _asbp_game_mode_base))))

(fn `Activate Lever`
  (params (`Hit Actor` :type "Actor Object Reference"))
  ;[1 1 1] 클릭한 액터가 Lever면 Activate Lever이벤트 실행
  (if (== `Hit Actor` (`self.Lever`))
    (bind _asbp_game_mode_base (cast `/Game/Blueprints/GameModeBase/BP_GameModeBase` (`GameplayStatics.GetGameMode`)))
    (if (not (`/Game/Blueprints/GameModeBase/BP_GameModeBase.lever` _asbp_game_mode_base))
      (`/Game/Blueprints/GameModeBase/BP_GameModeBase.Activate Lever` _asbp_game_mode_base)
      (`/Game/Blueprints/Item/BP_OldLever.RemoveOverlay` (`self.Lever`))
      (`self.Noise` (`self.K2_GetActorLocation`)))))

(fn `Get Item`
  (params (`Hit Actor` :type "Actor Object Reference"))
  (bind _returnvalue (`self.K2_GetActorLocation`))
  ;[1 1 1] 아이템 제거 및 획득 True로 변경
  (if (== `Hit Actor` (`self.Item`))
    (`self.K2_DestroyActor` (`self.Item`))
    (bind _asbp_game_mode_base (cast `/Game/Blueprints/GameModeBase/BP_GameModeBase` (`GameplayStatics.GetGameMode`)))
    (set `/Game/Blueprints/GameModeBase/BP_GameModeBase.item` true _asbp_game_mode_base)
    (`GameplayStatics.PlaySoundAtLocation` "/Game/Sounds/SOUND_KeyGet.SOUND_KeyGet" _returnvalue (struct) 1.0 1.0 0.0 "/Game/Sounds/SA_ZombieSound.SA_ZombieSound" null null null)
    (`self.Noise` _returnvalue)
    (elif (== `Hit Actor` (`self.bolt cutter`))
      (`self.K2_DestroyActor` (`self.bolt cutter`))
      (set `self.Get Bolt Cutter` true)
      (bind _asbp_game_mode_base_2 (cast `/Game/Blueprints/GameModeBase/BP_GameModeBase` (`GameplayStatics.GetGameMode`)))
      (set `/Game/Blueprints/GameModeBase/BP_GameModeBase.boltCutter` true _asbp_game_mode_base_2)
      (`GameplayStatics.PlaySoundAtLocation` "/Game/Sounds/SOUND_BoltCutterGet.SOUND_BoltCutterGet" (`self.K2_GetActorLocation`) (struct) 1.0 1.0 0.0 "/Game/Sounds/SA_ZombieSound.SA_ZombieSound" null null null))))

(fn `Is BoltCutter`
  (params (`Hit Actor` :type "Actor Object Reference"))
  (bind _bolt_cutter (`self.bolt cutter`))
  (bind _bolt_cutter_2 (`self.bolt cutter`))
  (if (`KismetSystemLibrary.IsValid` _bolt_cutter)
    (if (== `Hit Actor` _bolt_cutter)
      (`/Game/Blueprints/Item/BP_Item.ApplyOverlay` _bolt_cutter_2)
      (else
        (`/Game/Blueprints/Item/BP_Item.RemoveOverlay` _bolt_cutter_2)))))

(fn `Is Chain`
  (params (`Hit Actor` :type "Actor Object Reference"))
  (bind _chain (`self.chain`))
  (bind _chain_2 (`self.chain`))
  (if (`/Game/Blueprints/Item/BP_Chain.is remove?` _chain)
    _
    (elif (== `Hit Actor` _chain)
      (`/Game/Blueprints/Item/BP_Chain.ApplyOverlay` _chain_2)
      (else
        (`/Game/Blueprints/Item/BP_Chain.RemoveOverlay` _chain_2)))))

(fn `Is Item`
  (params (`Hit Actor` :type "Actor Object Reference"))
  (bind _item (`self.Item`))
  (bind _item_2 (`self.Item`))
  (if (`KismetSystemLibrary.IsValid` _item_2)
    (if (== `Hit Actor` _item_2)
      (`/Game/Blueprints/Item/BP_Item.ApplyOverlay` _item)
      (else
        (`/Game/Blueprints/Item/BP_Item.RemoveOverlay` _item)))))

(fn `Is Lever`
  (params (Actor :type "Actor Object Reference"))
  (bind _lever (`self.Lever`))
  (if (`KismetSystemLibrary.IsValid` _lever)
    (if (== Actor _lever)
      (bind _asbp_game_mode_base (cast `/Game/Blueprints/GameModeBase/BP_GameModeBase` (`GameplayStatics.GetGameMode`)))
      (if (not (`/Game/Blueprints/GameModeBase/BP_GameModeBase.lever` _asbp_game_mode_base))
        (`/Game/Blueprints/Item/BP_OldLever.ApplyOverlay` (`self.Lever`)))
      (else
        (`/Game/Blueprints/Item/BP_OldLever.RemoveOverlay` (`self.Lever`))))))

(fn `UserConstructionScript`)