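; Behavior tree task that sends a zombie enemy to investigate a heard location stored in a blackboard vector key.
; It plays a growl sound, then sets max or walk speed depending on the game mode's LastEvent flag.
; The enemy moves to a random reachable point near that location.
; On arrival it plays an idle montage and succeeds after it ends; a failed move fails the task.
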(event `self.ReceiveExecuteAI`
  (params (OwnerController :type "AIController Object Reference") (ControlledPawn :type "Pawn Object Reference"))
  (bind _asbp_enemy (cast `/Game/Blueprints/Enemy/BP_Enemy` ControlledPawn))
  (bind _audio (`/Game/Blueprints/Enemy/BP_Enemy.Audio` _asbp_enemy))
  (`AudioComponent.Stop` _audio)
  (`AudioComponent.SetSound` _audio "/Game/Sounds/MSS_ZombieGrowl.MSS_ZombieGrowl")
  (`AudioComponent.Play` _audio 0.0)
  (bind _asbp_game_mode_base (cast `/Game/Blueprints/GameModeBase/BP_GameModeBase` (`GameplayStatics.GetGameMode`)))
  (if (`/Game/Blueprints/GameModeBase/BP_GameModeBase.lastEvent` _asbp_game_mode_base)
    (`/Game/Blueprints/Enemy/BP_Enemy.MaxSpeed` _asbp_enemy)
    (else
      (`/Game/Blueprints/Enemy/BP_Enemy.WalkSpeed` _asbp_enemy)))
  (`|AIMoveTo` _asbp_enemy (`NavigationSystemV1.K2_GetRandomReachablePointInRadius` (`BlackboardComponent.GetValueAsVector` (`AIBlueprintHelperLibrary.GetBlackboard` OwnerController) (`self.Vector Key Name`)) 200.0 null null) null 100.0
    (:`OnSuccess`
      (bind _returnvalue (`Character.PlayAnimMontage` _asbp_enemy "/Game/Fab_Enemy/Zombie_Mutant/demo/animations/AM_Zombie_Idle.AM_Zombie_Idle" 1.0 "None"))
      (`KismetSystemLibrary.Delay` _returnvalue)
      (`self.FinishExecute` true))
    (:`OnFail`
      (`self.FinishExecute` false))))