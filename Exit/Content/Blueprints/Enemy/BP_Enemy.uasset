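; Enemy Blueprint that turns AI sight and hearing into Blackboard state, with events for switching movement speed.
; Sight targets the seen pawn and sets Howling; hearing stores the noise location unless already in Sight.
; Tick writes player distance to the attack key and counts down stimulus expiration before reverting to Patrol.
; On perception updates, LastDance forces Sight on the player without Howling if the GameMode's LastEvent is set.
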(event `IdleSpeed`
  (set `CharacterMovementComponent.MaxWalkSpeed` 0.0 (`self.CharacterMovement`)))

(event `WalkSpeed`
  (set `CharacterMovementComponent.MaxWalkSpeed` 250.0 (`self.CharacterMovement`)))

(event `RunSpeed`
  (bind _output_get (set `CharacterMovementComponent.MaxWalkSpeed` 300.0 (`self.CharacterMovement`))))

(event `self.ReceiveBeginPlay`
  (set `self.Blackboard` (`AIBlueprintHelperLibrary.GetBlackboard` null)))

(event `MaxSpeed`
  (bind _output_get (set `CharacterMovementComponent.MaxWalkSpeed` 410.0 (`self.CharacterMovement`))))

(event `self.AIPerception.OnPerceptionUpdated`
  (params (UpdatedActors :type "Array of Actor Object Reference (by ref)"))
  (`self.LastDance`)
  (for _array_element UpdatedActors
    (`|ExecutionSequence`
      (:`then_0`
        ;[1 1 1] 시야에 플레이어 감지 시 추격모드, 시야에 벗어나면 일정식간 이후 순찰 모드
        (bind (_senced _stimulus) (`self.Can Sence Actor` _array_element "NewEnumerator1"))
        (cast `Pawn` _array_element)
        (if _senced
          (`KismetSystemLibrary.PrintString` "sight sight" false true (struct :`R` 0.330762 :`G` 1.0 :`A` 1.0))
          (`self.HandleSightOn` _array_element)
          (else
            (set `self.OnTimer` true)
            (set `self.Timer` (`.ExpirationAge` (break `AIStimulus` _stimulus))))))
      (:`then_1`
        ;[1 1 1] 소리 반응
        (bind (_senced_2 _stimulus_2) (`self.Can Sence Actor` _array_element "NewEnumerator2"))
        (if _senced_2
          (`KismetSystemLibrary.PrintString` "hearing hearing" false true (struct :`R` 0.330762 :`G` 1.0 :`A` 1.0))
          (bind (_age _expirationage _strength _stimuluslocation) (break `AIStimulus` _stimulus_2))
          (`self.HandleHearingOn` _stimuluslocation)
          (set `self.OnTimer` false)
          (else
            (switch `/Game/Blueprints/Enemy/E_AISence` (cast `/Game/Blueprints/Enemy/E_AISence` (`BlackboardComponent.GetValueAsEnum` (`self.Blackboard`) (`self.State Key Name`)))
              (:`NewEnumerator0`
                _)
              (:`NewEnumerator2`
                _)
              (:`NewEnumerator4`
                _))
            (set `self.OnTimer` true)
            (set `self.Timer` _expirationage)
            (`KismetSystemLibrary.PrintString` "듣다말아" false)))))))

(event `self.ReceiveTick`
  (params (DeltaSeconds :type "Float (single-precision)"))
  ;[1 1 1] 시야, 소리에 반응 이후 순찰로 돌아가기
  (`self.SetAttackRange`)
  (`self.TimerPatrol` DeltaSeconds))

(fn `Can Sence Actor`
  (params (Actor :type "Actor Object Reference") (Sence :type "/Game/Blueprints/Enemy/E_AISence Enum" :default "NewEnumerator0"))
  (returns (Senced :type Boolean) (Stimulus :type "AIStimulus Structure"))
  (bind _info (`AIPerceptionComponent.GetActorsPerception` (`self.AIPerception`) Actor))
  (for _array_element (`.LastSensedStimuli` (break `ActorPerceptionBlueprintInfo` _info))
    (bind _returnvalue (`AIPerceptionSystem.GetSenseClassForStimulus` _array_element))
    (if (== _returnvalue (select `/Game/Blueprints/Enemy/E_AISence` Sence :`NewEnumerator1` "/Script/AIModule.AISense_Sight" :`NewEnumerator2` "/Script/AIModule.AISense_Hearing" :!type "Object Class Reference"))
      (return (`.bSuccessfullySensed` (break `AIStimulus` _array_element)) _array_element))))

(fn `HandleHearingOn`
  (params (`Hear Location` :type "Vector Structure"))
  (switch `/Game/Blueprints/Enemy/E_AISence` (cast `/Game/Blueprints/Enemy/E_AISence` (`BlackboardComponent.GetValueAsEnum` (`self.Blackboard`) (`self.State Key Name`)))
    (:`NewEnumerator0`
      _)
    (:`NewEnumerator2`
      _)
    (:`NewEnumerator4`
      _))
  (`BlackboardComponent.SetValueAsEnum` (`self.Blackboard`) (`self.State Key Name`) (enumliteral `/Game/Blueprints/Enemy/E_AISence` "NewEnumerator2"))
  (`BlackboardComponent.SetValueAsVector` (`self.Blackboard`) (`self.Vector Key Name`) `Hear Location`))

(fn `HandlePatrolOn`
  (switch `/Game/Blueprints/Enemy/E_AISence` (cast `/Game/Blueprints/Enemy/E_AISence` (`BlackboardComponent.GetValueAsEnum` (`self.Blackboard`) (`self.State Key Name`)))
    (:`NewEnumerator0`
      _)
    (:`NewEnumerator1`
      _)
    (:`NewEnumerator2`
      _)
    (:`NewEnumerator4`
      _))
  (`BlackboardComponent.SetValueAsEnum` (`self.Blackboard`) (`self.State Key Name`) (enumliteral `/Game/Blueprints/Enemy/E_AISence` "NewEnumerator4"))
  (`BlackboardComponent.SetValueAsObject` (`self.Blackboard`) (`self.Object Key Name`) null))

(fn `HandleSightOn`
  (params (ObjectValue :type "Object Object Reference"))
  (bind _blackboard (`self.Blackboard`))
  (switch `/Game/Blueprints/Enemy/E_AISence` (cast `/Game/Blueprints/Enemy/E_AISence` (`BlackboardComponent.GetValueAsEnum` (`self.Blackboard`) (`self.State Key Name`)))
    (:`NewEnumerator0`
      _)
    (:`NewEnumerator2`
      _)
    (:`NewEnumerator4`
      _))
  (set `self.OnTimer` false)
  (`BlackboardComponent.SetValueAsEnum` (`self.Blackboard`) (`self.State Key Name`) (enumliteral `/Game/Blueprints/Enemy/E_AISence` "NewEnumerator1"))
  (`BlackboardComponent.SetValueAsObject` _blackboard (`self.Object Key Name`) ObjectValue)
  (`BlackboardComponent.SetValueAsBool` _blackboard "Howling" true)
  (return))

(fn `LastDance`
  (bind _blackboard (`self.Blackboard`))
  (bind _asbp_game_mode_base (cast `/Game/Blueprints/GameModeBase/BP_GameModeBase` (`GameplayStatics.GetGameMode`)))
  (if (`/Game/Blueprints/GameModeBase/BP_GameModeBase.lastEvent` _asbp_game_mode_base)
    (set `self.OnTimer` false)
    (`BlackboardComponent.SetValueAsEnum` _blackboard (`self.State Key Name`) (enumliteral `/Game/Blueprints/Enemy/E_AISence` "NewEnumerator1"))
    (`BlackboardComponent.SetValueAsBool` _blackboard "Howling" false)
    (bind _asbp_player (cast `/Game/Blueprints/BP_Player` (`GameplayStatics.GetPlayerPawn` 0)))
    (`BlackboardComponent.SetValueAsObject` (`self.Blackboard`) (`self.Object Key Name`) _asbp_player)))

(fn `SetAttackRange`
  (`BlackboardComponent.SetValueAsFloat` (`self.Blackboard`) (`self.Attack Key Name`) (`self.GetDistanceTo` (`GameplayStatics.GetPlayerPawn` 0))))

(fn `TimerPatrol`
  (params (B :type "Float (double-precision)"))
  (if (`self.OnTimer`)
    (bind _output_get (set `self.Timer` (- (`self.Timer`) B)))
    (if (< _output_get 0.0)
      (`KismetSystemLibrary.PrintString` "nono Sight" false true (struct :`R` 0.330762 :`G` 1.0 :`A` 1.0))
      (`self.HandlePatrolOn`)
      (set `self.OnTimer` false)
      (set `self.IsSight` false))))

(fn `UserConstructionScript`)