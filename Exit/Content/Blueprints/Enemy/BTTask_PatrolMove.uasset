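; Behavior tree task that makes a zombie enemy wander to a random nearby spot while patrolling.
; It restarts the enemy's audio with the patrol sound and switches it to walk speed.
; It then moves the pawn to a random reachable point within a radius of its current location, finishing with success or failure according to the move result.
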(event `self.ReceiveExecuteAI`
  (params (OwnerController :type "AIController Object Reference") (ControlledPawn :type "Pawn Object Reference"))
  (bind _asbp_enemy (cast `/Game/Blueprints/Enemy/BP_Enemy` ControlledPawn))
  (bind _audio (`/Game/Blueprints/Enemy/BP_Enemy.Audio` _asbp_enemy))
  (`AudioComponent.Stop` _audio)
  (`AudioComponent.SetSound` _audio "/Game/Sounds/MSS_ZombiePatrol.MSS_ZombiePatrol")
  (`AudioComponent.Play` _audio 0.0)
  (`/Game/Blueprints/Enemy/BP_Enemy.WalkSpeed` _asbp_enemy)
  (`|AIMoveTo` _asbp_enemy (`NavigationSystemV1.K2_GetRandomReachablePointInRadius` (`Actor.K2_GetActorLocation` _asbp_enemy) 3000.0 null null) null 100.0
    (:`OnSuccess`
      (`self.FinishExecute` true))
    (:`OnFail`
      (`self.FinishExecute` false))))